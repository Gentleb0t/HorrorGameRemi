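; BP_FLickering_light is a flickering spotlight for the horror game, paired with an Elec component that is re-activated during the flicker.
; From BeginPlay, a chain of delays endlessly loops, snapping the spotlight intensity between off and full in two quick blinks, then holding it lit briefly before repeating.
; The pattern is fixed and hard-coded, with no randomness, timeline or stop condition.
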(event EventBeginPlay
  (bind _spotlight (Variables|Default|GetSpotLight))
  (Rendering|Components|Light|SetIntensity (Variables|Default|GetSpotLight) 0.0 :!label _label)
  (Utilities|FlowControl|Delay 0.1)
  (Components|Activation|Activate (Variables|Default|GetElec) true)
  (Rendering|Components|Light|SetIntensity (Variables|Default|GetSpotLight) 2.5e+03)
  (Utilities|FlowControl|Delay 0.1)
  (Components|Activation|Activate (Variables|Default|GetElec) true)
  (Rendering|Components|Light|SetIntensity _spotlight 0.0)
  (Utilities|FlowControl|Delay 0.1)
  (Rendering|Components|Light|SetIntensity _spotlight 2.5e+03)
  (Utilities|FlowControl|Delay 1.5)
  (goto _label))

(fn ConstructionScript)