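; BP_Faulty_Double_Door is a malfunctioning horror-game double door that jitters until the player fixes it.
; From BeginPlay, a self-restarting timeline slides both panels slightly, activating Niagara effects and calling a 2D sound on each update.
; Interaction checks the third-person character's HasPressedButton flag, then sets DoorFixed to end the loop.
; A second timeline slides the panels wide open, hides the icon, marks the door open and clears the flag.
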(event EventBeginPlay
  ;[0 0.024 0.1] Animation for the doors
  (bind _faulty_door (Timeline|Open%20Door Play)
    (:Update
      (Utilities|FlowControl|Sequence
        (:then_0
          (Transformation|SetRelativeLocation (Variables|Default|GetDoor%202) (Math|Vector|MakeVector -18.0 (Math|Float|Lerp 49.0 6e+01 _faulty_door) -17.0) false false)
          (Components|Activation|Activate (Variables|Default|GetNiagara1) false))
        (:then_1
          (Transformation|SetRelativeLocation (Variables|Default|GetDoor) (Math|Vector|MakeVector -1.0 (Math|Float|Lerp -234.0 -259.0 _faulty_door) -17.0) false false)
          (Components|Activation|Activate (Variables|Default|GetNiagara) false))
        (:then_2
          (Audio|PlaySound2D 0 1.0 1.0 0.0 0 0))))
    (:Finished
      (if (Variables|Default|GetDoor%20fixed)
        (Timeline|Open%20Door Stop)
        (else
          (Timeline|Open%20Door PlayFromStart))))))

(event EventInteraction
  (bind _asbp_third_person_character (Utilities|Casting|CastToBP_ThirdPersonCharacter (Game|GetPlayerCharacter 0)))
  (if (Variables|/Game/GameHorror/BP_And_UI/Blueprint/BP_ThirdPersonCharacter.BP_ThirdPersonCharacter_C|GetHas%20Pressed%20Button? _asbp_third_person_character)
    (Variables|Default|SetDoor%20fixed true)
    (bind _open___close_door (Timeline|Timeline Play)
      (:Update
        (Utilities|FlowControl|Sequence
          (:then_0
            (Transformation|SetRelativeLocation (Variables|Default|GetDoor%202) (Math|Vector|MakeVector -18.0 (Math|Float|Lerp 49.0 178.0 _open___close_door) -17.0) false false)
            (Rendering|SetVisibility (Variables|Default|GetIcon) false false)
            (Variables|Default|SetIs%20Door%20Open? true)
            (Variables|/Game/GameHorror/BP_And_UI/Blueprint/BP_ThirdPersonCharacter.BP_ThirdPersonCharacter_C|SetHas%20Pressed%20Button? _asbp_third_person_character false))
          (:then_1
            (Transformation|SetRelativeLocation (Variables|Default|GetDoor) (Math|Vector|MakeVector -1.0 (Math|Float|Lerp -234.0 -358.0 _open___close_door) -17.0) false false)
            (Variables|Default|SetIs%20Door%20Open? true)))))))

(fn ConstructionScript)