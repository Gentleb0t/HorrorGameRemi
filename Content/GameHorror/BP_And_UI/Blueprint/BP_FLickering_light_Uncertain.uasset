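; Flickering spotlight actor for the horror game that pairs its light flicker with an electrical effect component, Elec.
; BeginPlay starts an endless Delay-driven loop that steps the SpotLight between dead, fixed mid-sequence and peak intensities.
; Elec is re-activated with reset just before two of the intensity changes.
; Timing and the dead and peak levels come from variables, with no randomization in the graph.
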(event EventBeginPlay
  (bind _spotlight (Variables|Default|GetSpotLight))
  (Rendering|Components|Light|SetIntensity (Variables|Default|GetSpotLight) (Variables|Default|GetDeadIntensity) :!label _label)
  (Utilities|FlowControl|Delay (Variables|Default|GetFlicker%20Delay))
  (Components|Activation|Activate (Variables|Default|GetElec) true)
  (Rendering|Components|Light|SetIntensity (Variables|Default|GetSpotLight) 2.5e+03)
  (Utilities|FlowControl|Delay (Variables|Default|GetFlickerDelay2))
  (Components|Activation|Activate (Variables|Default|GetElec) true)
  (Rendering|Components|Light|SetIntensity _spotlight (Variables|Default|GetDeadIntensity))
  (Utilities|FlowControl|Delay (Variables|Default|GetFlicker%20Delay))
  (Rendering|Components|Light|SetIntensity _spotlight (Variables|Default|GetPeakIntensity))
  (Utilities|FlowControl|Delay (Variables|Default|GetReset))
  (goto _label))

(fn ConstructionScript)