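; BP_Lamp_A is a lamp actor with a spot light that can flicker like a faulty fixture.
; When IsFaulty is set, BeginPlay starts an endless Delay-driven loop that steps the SpotLight between dead, intermediate and peak intensities, activating the Elec effect component during the flicker.
; Variables set the delays and the dead and peak levels, while the intermediate level is hardcoded.
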(event EventBeginPlay
  (bind _spotlight (Variables|Default|GetSpotLight))
  (if (Variables|Default|GetIsFaulty)
    (Rendering|Components|Light|SetIntensity (Variables|Default|GetSpotLight) (Variables|Default|GetDeadIntensity) :!label _label)
    (Utilities|FlowControl|Delay (Variables|Default|GetFlicker%20Delay))
    (Components|Activation|Activate (Variables|Default|GetElec) true)
    (Rendering|Components|Light|SetIntensity (Variables|Default|GetSpotLight) 2.5e+03)
    (Utilities|FlowControl|Delay (Variables|Default|GetFlickerDelay2))
    (Components|Activation|Activate (Variables|Default|GetElec) true)
    (Rendering|Components|Light|SetIntensity _spotlight (Variables|Default|GetDeadIntensity))
    (Utilities|FlowControl|Delay (Variables|Default|GetFlicker%20Delay))
    (Rendering|Components|Light|SetIntensity _spotlight (Variables|Default|GetPeakIntensity))
    (Utilities|FlowControl|Delay (Variables|Default|GetReset))
    (goto _label)))

(event Collision|EventActorBeginOverlap
  (params (OtherActor :type Actor%20Object%20Reference)))

(event EventTick
  (params (DeltaSeconds :type Float%20%28single-precision%29)))

(fn ConstructionScript)